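; TowerBP is a tower actor that fires at NPCs entering its range.
; On BeginPlay it reads the StandardTower row from TowerDataTable, stores it, and sets the tower mesh from it.
; When an NPC_Basic begins overlapping the range sphere, it spawns one TowerProjectile at the tower's transform with that NPC as target.
; Firing is triggered only by the overlap event, with no timer or repeat fire.
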(event `self.Sphere.OnComponentBeginOverlap`
  (params (OverlappedComponent :type "PrimitiveComponent Object Reference") (OtherActor :type "Actor Object Reference") (OtherComp :type "PrimitiveComponent Object Reference") (OtherBodyIndex :type Integer) (bFromSweep :type Boolean) (SweepResult :type "HitResult Structure (by ref)"))
  ;[1 1 1] If NPC in range, Spawn Projectile from tower
  (bind _asnpc_basic (cast `/Game/AI/NPC_Basic` OtherActor))
  (`|SpawnActorFromClass` "/Game/Tower/TowerProjectile.TowerProjectile_C" (`self.GetTransform`) "AlwaysSpawn" "OverrideRootScale" null _asnpc_basic null))

(event `self.ReceiveBeginPlay`
  ;[1 1 1] On Begin
  ; Get tower data from table, store in var
  (bind _returnvalue (`|GetDataTableRow` "/Game/Tower/TowerDataTable.TowerDataTable" "StandardTower")
    (:`then`
      (set `self.TowerStruct` _returnvalue)
      (`self.TowerInit`))))

(event `TowerInit`
  ;[1 1 1] Create Tower
  (`StaticMeshComponent.SetStaticMesh` (`self.TowerMesh`) (`.Mesh_16_8C3CEDFA4E271E67C9DA62867FEF8C09` (break `/Game/Tower/TowerStruct` (`self.TowerStruct`)))))

(fn `UserConstructionScript`)