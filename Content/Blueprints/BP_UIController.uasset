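; BP_UIController is an actor that toggles the pause menu on and off.
; On BeginPlay it finds the first HUD_01 in the world and caches it as HUDRef.
; The P key and the Pause Menu Toggle input action share one path that flips the HUD's PauseMenuRef widget between Visible and Hidden, printing debug strings.
; It changes only widget visibility and does not pause the game.
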(event `self.ReceiveBeginPlay`
  (bind _outactors (`GameplayStatics.GetAllActorsOfClass` "/Game/UI/HUD_01.HUD_01_C"))
  (set `self.HUD_Ref` (`|GetArrayItem` _outactors)))

(event `Key|P`
  (params (Key :type "Key Structure"))
  (bind _pausemenuref (`/Game/UI/HUD_01.PauseMenuRef` (`self.HUD_Ref`)))
  ;[1 1 1] Pause Menu
  (:`Pressed`
    (`KismetSystemLibrary.PrintString` "Space pressed" false false :!label _label)
    (if (`Widget.IsVisible` _pausemenuref)
      (`Widget.SetVisibility` _pausemenuref "Hidden")
      (`KismetSystemLibrary.PrintString` "pause menu hidden")
      (else
        (`Widget.SetVisibility` _pausemenuref "Visible")
        (`KismetSystemLibrary.PrintString` "pause menu visible")))))

(event `InputAction|Pause Menu Toggle`
  (params (Key :type "Key Structure"))
  ;[1 1 1] Pause Menu
  (:`Pressed`
    (goto _label)))

(fn `UserConstructionScript`)