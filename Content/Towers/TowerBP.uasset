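; Team-based defence tower that fires projectiles at enemy NPC ships within range, using North or South allegiance.
; BeginPlay loads mesh, range, damage and fire rate from a data table row.
; Range-sphere overlaps set or clear the target, while Tick fires on cooldown or runs throttled sphere traces when untargeted.
; ClosestTargetCalculation filters trace hits by team, but clears its candidate instead of switching when a closer one appears.
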(event `Shoot`
  (bind (_name _damage _range _firerate) (break `/Game/Towers/TowerStruct` (`self.TowerStruct`)))
  (set `self.CooldownActive` true)
  (`|SpawnActorFromClass` "/Game/Towers/TowerProjectile.TowerProjectile_C" (`self.GetTransform`) "AlwaysSpawn" "OverrideRootScale" null _damage (`self.TowerTarget`) null)
  (`GameplayStatics.PlaySoundAtLocation` "/Game/Audio/SFX/TowerFire_Cannon+1_Cue.TowerFire_Cannon+1_Cue" (`self.K2_GetActorLocation`) (struct) 1.0 1.0 0.0 null null null)
  (`KismetSystemLibrary.Delay` _firerate)
  (set `self.CooldownActive` false))

(event `self.ReceiveTick`
  (params (DeltaSeconds :type "Float (single-precision)"))
  (`/Engine/EditorBlueprintResources/StandardMacros.IsValid` (`self.TowerTarget`)
    (:`Is Valid`
      (if (not (`self.CooldownActive`))
        (`self.Shoot`)))
    (:`Is Not Valid`
      (if (not (`self.TargetCheckCooldownActive`))
        (`self.CheckForNewTarget`)))))

(event `CheckForNewTarget`
  (bind _returnvalue (`self.K2_GetActorLocation`))
  (set `self.TargetCheckCooldownActive` true)
  (bind (_outhits _returnvalue_2) (`KismetSystemLibrary.SphereTraceMultiForObjects` _returnvalue (- _returnvalue (0.0 0.0 1.0)) (`.Range_14_641CF504479D72B8B8799B996C19D074` (break `/Game/Towers/TowerStruct` (`self.TowerStruct`))) (`|MakeArray` "ObjectTypeQuery3" :!type "EObjectTypeQuery Enum")))
  (if _returnvalue_2
    (bind _target (`self.ClosestTargetCalculation` _outhits))
    (`/Engine/EditorBlueprintResources/StandardMacros.IsValid` _target
      (:`Is Valid`
        (set `self.TowerTarget` _target))
      (:`Is Not Valid`
        _)))
  (`KismetSystemLibrary.Delay` 0.25)
  (set `self.TargetCheckCooldownActive` false))

(event `self.SphereRange.OnComponentBeginOverlap`
  (params (OverlappedComponent :type "PrimitiveComponent Object Reference") (OtherActor :type "Actor Object Reference") (OtherComp :type "PrimitiveComponent Object Reference") (OtherBodyIndex :type Integer) (bFromSweep :type Boolean) (SweepResult :type "HitResult Structure (by ref)"))
  ;[1 1 1] If NPC in range, Spawn Projectile from tower
  (if (`KismetStringLibrary.EqualEqual_StrStr` (`KismetSystemLibrary.GetObjectName` OtherComp) "TargetContact")
    ;[1 1 1] if we dont have a valid target get a new one
    (`/Engine/EditorBlueprintResources/StandardMacros.IsValid` (`self.TowerTarget`)
      (:`Is Not Valid`
        (bind _asnpc_ship_character (cast `/Game/Ships/NPC_ShipCharacter` OtherActor))
        ;[1 1 1] is this a nth tower?
        (if (`self.NorthTower`)
          (bind _teamname (`/Game/Ships/NPC_ShipCharacter.TeamName` _asnpc_ship_character))
          ;[1 1 1] is enemy?
          (if (`KismetStringLibrary.EqualEqual_StrStr` _teamname "South")
            (set `self.TowerTarget` _asnpc_ship_character :!label _label))
          (elif (`KismetStringLibrary.EqualEqual_StrStr` _teamname "North")
            (goto _label)))))))

(event `self.SphereRange.OnComponentEndOverlap`
  (params (OverlappedComponent :type "PrimitiveComponent Object Reference") (OtherActor :type "Actor Object Reference") (OtherComp :type "PrimitiveComponent Object Reference") (OtherBodyIndex :type Integer))
  ;[1 1 1] If target leaves sphere set to null
  (if (`KismetStringLibrary.EqualEqual_StrStr` (`KismetSystemLibrary.GetObjectName` OtherComp) "TargetContact")
    (if (== OtherActor (`self.TowerTarget`))
      (set `self.TowerTarget` null))))

(event `self.ReceiveBeginPlay`
  ;[1 1 1] On Begin
  ; Get tower data from table, store in var
  (bind _returnvalue (`|GetDataTableRow` "/Game/Towers/TowerDataTable.TowerDataTable" "PirateTower")
    (:`then`
      (set `self.TowerStruct` _returnvalue)
      (`self.TowerInit`))))

(event `TowerInit`
  (bind (_name _damage _range _firerate _mesh) (break `/Game/Towers/TowerStruct` (`self.TowerStruct`)))
  ;[1 1 1] Create Tower
  (`StaticMeshComponent.SetStaticMesh` (`self.TowerMesh`) _mesh)
  (`SphereComponent.SetSphereRadius` (`self.SphereRange`) _range true))

(fn `ClosestTargetCalculation`
  (params (HitResults :type "Array of HitResult Structure"))
  (returns (Target :type "/Game/Ships/NPC_ShipCharacter Object Reference"))
  (locals (TempTarget :type "/Game/Ships/NPC_ShipCharacter Object Reference") (TempDistance :type "Float (double-precision)" :default 0.0))
  ;[-0.08489 1 1] Checks all hits
  ; If npc ship,
  ; Return closest enemy
  (for _array_element HitResults
    (bind (_bblockinghit _binitialoverlap _time _distance _location _impactpoint _normal _impactnormal _physmat _hitactor) (`GameplayStatics.BreakHitResult` _array_element))
    (bind _asnpc_ship_character (cast `/Game/Ships/NPC_ShipCharacter` _hitactor))
    ;;[1 1 1] Check tower vs enemy teams
    ;;;[1 1 1] Is Nth Tower
    (if (`self.NorthTower`)
      (bind _teamname (`/Game/Ships/NPC_ShipCharacter.TeamName` _asnpc_ship_character))
      ;;;[1 1 1] Sth Enemy
      (if (`KismetStringLibrary.EqualEqual_StrStr` _teamname "South")
        (`/Engine/EditorBlueprintResources/StandardMacros.IsValid` (`local.TempTarget`) :!label _label
          (:`Is Valid`
            (bind _returnvalue (`KismetMathLibrary.VSize` (- (`self.K2_GetActorLocation`) (`self.K2_GetActorLocation` _hitactor))))
            (if (< _returnvalue (`local.TempDistance`))
              (set `local.TempTarget` null)
              (set `local.TempDistance` _returnvalue)))
          (:`Is Not Valid`
            (set `local.TempTarget` _asnpc_ship_character)
            (set `local.TempDistance` _returnvalue))))
      (else
        ;;;[1 1 1] Nth Enemy
        (if (`KismetStringLibrary.EqualEqual_StrStr` _teamname "North")
          (goto _label)))))
  (return (`local.TempTarget`)))

(fn `UserConstructionScript`)