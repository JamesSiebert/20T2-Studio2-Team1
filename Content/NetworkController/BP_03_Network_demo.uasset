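; Networking demo actor that labels itself "Server" or "Client" by authority and rotates a sphere.
; On authority, a looping timer calls FixRotation to pick a new random RotationValue.
; Every instance applies RotationValue to the sphere's world rotation on Tick; the file does not show whether that variable replicates.
; A disconnected Delay node leading to the rotation update never runs.
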(event `self.ReceiveBeginPlay`
  (bind _textrender (`self.TextRender`))
  (`/Engine/EditorBlueprintResources/ActorMacros.Switch Has Authority`
    (:`Authority`
      (`TextRenderComponent.K2_SetText` _textrender (`KismetTextLibrary.Conv_StringToText` "Server"))
      (`KismetSystemLibrary.K2_SetTimer` null "FixRotation" 0.8 true))
    (:`Remote`
      (`TextRenderComponent.K2_SetText` _textrender (`KismetTextLibrary.Conv_StringToText` "Client")))))

(event `self.ReceiveTick`
  (params (DeltaSeconds :type "Float (single-precision)"))
  (`SceneComponent.K2_SetWorldRotation` (`self.Sphere`) (`self.RotationValue`) false false))

(fn `FixRotation`
  (set `self.RotationValue` (`KismetMathLibrary.RandomRotator` false))
  (return))

(fn `UserConstructionScript`)