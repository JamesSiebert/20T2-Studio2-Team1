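; BP_SharedData is a data holder for the North and South teams, storing each side's bank balance, team color and player spawn point.
; Getters expose all three values per team, while only the bank balances have functions to set, add and deduct.
; Deductions fail and return false when the amount exceeds the balance, unless a Force flag skips the check and lets the balance go negative.
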(fn `AddTo_NorthBankBalance`
  (params (Amount :type "Float (double-precision)"))
  (returns (Success :type Boolean))
  (set `self.NorthBank` (+ (`self.NorthBank`) Amount))
  (return true))

(fn `AddTo_SouthBankBalance`
  (params (Amount :type "Float (double-precision)"))
  (returns (Success :type Boolean))
  (set `self.SouthBank` (+ (`self.SouthBank`) Amount))
  (return true))

(fn `Deduct_NorthBankBalance`
  (params (Amount :type "Float (double-precision)") (Force :type Boolean))
  (returns (Success :type Boolean))
  (if Force
    _
    (elif (<= Amount (`self.NorthBank`))
      _
      (else
        (return false))))
  (set `self.NorthBank` (- (`self.NorthBank`) Amount))
  (return true))

(fn `Deduct_SouthBankBalance`
  (params (Amount :type "Float (double-precision)") (Force :type Boolean))
  (returns (Success :type Boolean))
  (if Force
    _
    (elif (<= Amount (`self.SouthBank`))
      _
      (else
        (return false))))
  (set `self.SouthBank` (- (`self.SouthBank`) Amount))
  (return true))

(fn `Get_NorthBankBalance`
  (returns (Balance :type "Float (double-precision)"))
  (return (`self.NorthBank`)))

(fn `Get_NorthColor`
  (returns (Color :type String))
  (return (`self.NorthTeamColor`)))

(fn `Get_NorthPlayerSpawnPoint`
  (returns (Location :type "Vector Structure"))
  (return (`self.NorthPlayerSpawnPoint`)))

(fn `Get_SouthBankBalance`
  (returns (Balance :type "Float (double-precision)"))
  (return (`self.SouthBank`)))

(fn `Get_SouthColor`
  (returns (Color :type String))
  (return (`self.SouthTeamColor`)))

(fn `Get_SouthPlayerSpawnPoint`
  (returns (Location :type "Vector Structure"))
  (return (`self.SouthPlayerSpawnPoint`)))

(fn `Set_NorthBankBalance`
  (params (Balance :type "Float (double-precision)"))
  (returns (Success :type Boolean))
  (set `self.NorthBank` Balance)
  (return true))

(fn `Set_SouthBankBalance`
  (params (Balance :type "Float (double-precision)"))
  (returns (Success :type Boolean))
  (set `self.SouthBank` Balance)
  (return true))

(fn `UserConstructionScript`)